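; BP_MyPawn is a pawn that manages two cable components around a loaded bird projectile, apparently the bands of a slingshot.
; On BeginPlay and on the AttachCable event, AttachCableBP attaches both cable ends to ProjectilAnchor, whether or not LoadedBird is valid.
; The nodes that would attach the cables directly to LoadedBird are disconnected.
; Tick prints the name of each cable's attached actor for debugging.
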(event `self.AttachCable`
  (`self.AttachCableBP`))

(event `self.ReceiveBeginPlay`
  (`self.AttachCableBP`))

(event `self.ReceiveTick`
  (params (DeltaSeconds :type "Float (single-precision)"))
  (`KismetSystemLibrary.PrintString` (`KismetSystemLibrary.GetDisplayName` (`CableComponent.GetAttachedActor` (`self.Cable1`))))
  (`KismetSystemLibrary.PrintString` (`KismetSystemLibrary.GetDisplayName` (`CableComponent.GetAttachedActor` (`self.Cable`)))))

(fn `AttachCableBP`
  (bind _projectilanchor (`self.ProjectilAnchor`))
  (`/Engine/EditorBlueprintResources/StandardMacros.IsValid` (`self.LoadedBird`)
    (:`Is Valid`
      _)
    (:`Is Not Valid`
      _))
  (`CableComponent.SetAttachEndToComponent` (`self.Cable`) _projectilanchor "None")
  (`CableComponent.SetAttachEndToComponent` (`self.Cable1`) _projectilanchor "None")
  (return))

(fn `UserConstructionScript`)